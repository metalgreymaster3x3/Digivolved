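; Digimon AI controller, named for fight-back behavior, that starts a creature's behavior tree when play begins.
; On the server it runs the configured behavior tree, then seeds the blackboard with attack destination offset, rotation range and interval values from the PrimalDinoAIController.
; The construction script only calls the parent's.
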(event `self.ReceiveBeginPlay`
  (bind _asprimaldinoaicontroller (cast `PrimalDinoAIController` self))
  (bind _returnvalue (`self.GetAttackInterval` _asprimaldinoaicontroller))
  (bind _returnvalue_2 (`self.GetAttackRotationRangeDegrees` _asprimaldinoaicontroller))
  (if (`self.HasAuthority` _asprimaldinoaicontroller)
    (`self.RunBehaviorTree` (`PrimalDinoAIController.BehaviourTree` _asprimaldinoaicontroller))
    (bind _returnvalue_3 (`AIBlueprintHelperLibrary.GetBlackboard` _asprimaldinoaicontroller))
    (`BlackboardComponent.SetValueAsFloat` _returnvalue_3 "AttackDestinationOffsetKey" (`PrimalDinoAIController.AttackDestinationOffset` _asprimaldinoaicontroller))
    (`BlackboardComponent.SetValueAsFloat` _returnvalue_3 "AttackRotationRangeKey" _returnvalue_2)
    (`BlackboardComponent.SetValueAsFloat` _returnvalue_3 "AttackIntervalKey" _returnvalue)))

(fn `UserConstructionScript`
  (`parent.UserConstructionScript`))