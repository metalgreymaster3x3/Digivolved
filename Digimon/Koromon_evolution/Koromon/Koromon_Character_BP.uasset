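; Koromon creature Blueprint for a Digimon mod, providing the creature's melee and ranged attacks.
; BPDoAttack selects the attack by index: after a short delay, melee applies radial damage at the Melee component, while ranged launches a projectile from the Ranged component.
; Inventory-based evolution into Agumon or Black Agumon, consuming DataGEN and Viral sequence items, is present but disconnected, and both tick events are empty.
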(event `Ranged_ATTK`
  (bind _ranged (`self.Ranged`))
  (bind _returnvalue (`SceneComponent.K2_GetComponentRotation` _ranged))
  (`KismetSystemLibrary.Delay` 0.3)
  (bind _returnvalue_2 (`|SpawnActorFromClass` "/Game/Mods/Digivolved/Digimon/Koromon_evolution/Koromon/Projectiles/Proj_KoromonNew.Proj_KoromonNew_C" (`KismetMathLibrary.MakeTransform` (`SceneComponent.K2_GetComponentLocation` _ranged) _returnvalue)))
  (`ShooterProjectile.BPInitVelocity` _returnvalue_2 (`KismetMathLibrary.GetForwardVector` _returnvalue)))

(event `self.ReceiveTick`
  (params (DeltaSeconds :type "Float (single-precision)")))

(event `On tick`)

(event `Melee_ATTK`
  (`KismetSystemLibrary.Delay` 0.3)
  (`GameplayStatics.ApplyRadialDamage` (`self.MeleeDmg`) (`SceneComponent.K2_GetComponentLocation` (`self.Melee`)) 100.0 (`self.DmgTypeMelee`) (`|MakeArray` self :!type "Actor Object Reference") self))

(fn `BPDoAttack`
  (params (AttackIndex :type Integer))
  (if (== AttackIndex 1)
    (`self.Ranged_ATTK`)
    (elif (== AttackIndex 0)
      (`self.Melee_ATTK`))))

(fn `UserConstructionScript`
  (`parent.UserConstructionScript`))