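; Palmon creature Blueprint providing a melee and a ranged attack, with BPDoAttack choosing between them by attack index.
; The melee event waits on a fixed delay, then deals radial damage around the Melee component, ignoring itself.
; The ranged event waits on a shorter delay, then spawns a rocket projectile at the Ranged component and launches it along that component's forward vector.
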(event `Ranged_attack`
  (bind _ranged (`self.Ranged`))
  (bind _returnvalue (`SceneComponent.K2_GetComponentRotation` _ranged))
  (`KismetSystemLibrary.Delay` 0.414)
  (bind _returnvalue_2 (`|SpawnActorFromClass` "/Game/PrimalEarth/Test/ProjRocket.ProjRocket_C" (`KismetMathLibrary.MakeTransform` (`SceneComponent.K2_GetComponentLocation` _ranged) _returnvalue)))
  (`ShooterProjectile.BPInitVelocity` _returnvalue_2 (`KismetMathLibrary.GetForwardVector` _returnvalue)))

(event `Melee_Attack`
  (`KismetSystemLibrary.Delay` 0.887)
  (`GameplayStatics.ApplyRadialDamage` (`self.Melee Damage`) (`SceneComponent.K2_GetComponentLocation` (`self.Melee`)) 100.0 (`self.Melee_DamageType`) (`|MakeArray` self :!type "Actor Object Reference") self))

(fn `BPDoAttack`
  (params (AttackIndex :type Integer))
  (if (== AttackIndex 1)
    (`self.Ranged_attack`)
    (elif (== AttackIndex 0)
      (`self.Melee_Attack`))))

(fn `UserConstructionScript`
  (`parent.UserConstructionScript`))