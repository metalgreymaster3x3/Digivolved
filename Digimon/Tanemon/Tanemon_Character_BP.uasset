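; Tanemon creature Blueprint for a Digimon mod, adding a ranged plant-projectile attack.
; Attack index 0 in BPDoAttack calls FireProjectil, which waits briefly, spawns Tanemon_ProjDefPlant at Box1's transform and launches it along that box's forward vector.
; Tick events are empty; unconnected leftover nodes hold a timed OnTick call and an item-cost check that spawns a Tane-to-Pal actor, apparently for evolution.
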(event `self.ReceiveTick`
  (params (DeltaSeconds :type "Float (single-precision)")))

(event `On tick`)

(event `FireProjectil`
  (bind _box1 (`self.Box1`))
  (bind _returnvalue (`SceneComponent.K2_GetComponentRotation` _box1))
  (`KismetSystemLibrary.Delay` 0.834)
  (bind _returnvalue_2 (`|SpawnActorFromClass` "/Game/Mods/Digivolved/Digimon/Tanemon/Proj/Tanemon_ProjDefPlant.Tanemon_ProjDefPlant_C" (`KismetMathLibrary.MakeTransform` (`SceneComponent.K2_GetComponentLocation` _box1) _returnvalue)))
  (`ShooterProjectile.BPInitVelocity` _returnvalue_2 (`KismetMathLibrary.GetForwardVector` _returnvalue)))

(fn `BPDoAttack`
  (params (AttackIndex :type Integer))
  (if (== AttackIndex 0)
    (`self.FireProjectil`)))

(fn `UserConstructionScript`
  (`parent.UserConstructionScript`))