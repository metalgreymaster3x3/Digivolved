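; Character Blueprint for the Tsunomon Digimon creature, holding a draft item-gated evolution, apparently into Gabumon.
; The evolution logic checks its inventory for at least three DataGENSequence consumables, removes one and spawns the Tsuno_to_Gabu actor at its transform.
; That logic and a delayed OnTick call are disconnected and never run; both tick events are empty, and construction only calls the parent.
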(event `self.ReceiveTick`
  (params (DeltaSeconds :type "Float (single-precision)")))

(event `On tick`)

(fn `UserConstructionScript`
  (`parent.UserConstructionScript`))