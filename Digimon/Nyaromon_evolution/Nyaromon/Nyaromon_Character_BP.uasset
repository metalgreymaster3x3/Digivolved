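; Character Blueprint for Nyaromon, a creature in a Digimon evolution line, that supplies its two melee attacks.
; BPDoAttack maps attack index 0 to a bite and index 1 to a swing, each fired through its own event.
; After a short delay timed per attack, each event applies radial damage from its own box component with its own damage amount, radius and damage type, ignoring itself.
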(event `FireProjectil`
  (`KismetSystemLibrary.Delay` 0.072)
  (`GameplayStatics.ApplyRadialDamage` (`self.MeleeDmgBite`) (`SceneComponent.K2_GetComponentLocation` (`self.Box1`)) 100.0 (`self.DmgTypeBite`) (`|MakeArray` self :!type "Actor Object Reference") self))

(event `FireProjecti2`
  (`KismetSystemLibrary.Delay` 0.3)
  (`GameplayStatics.ApplyRadialDamage` (`self.MeleeDmgSwing`) (`SceneComponent.K2_GetComponentLocation` (`self.Box2`)) 200.0 (`self.DmgTypeSwing`) (`|MakeArray` self :!type "Actor Object Reference") self))

(fn `BPDoAttack`
  (params (AttackIndex :type Integer))
  (if (== AttackIndex 0)
    (`self.FireProjectil`)
    (elif (== AttackIndex 1)
      (`self.FireProjecti2`))))

(fn `UserConstructionScript`
  (`parent.UserConstructionScript`))