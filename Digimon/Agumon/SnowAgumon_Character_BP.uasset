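; SnowAgumon creature Blueprint that implements two attacks, a melee hit and a snow projectile, selected by index in BPDoAttack.
; The melee attack waits briefly, then applies radial damage around Box2 using MeleeDmg, ignoring itself.
; The ranged attack waits longer, then spawns ProjSnow_SnowAgumon at Box1 and launches it along that box's forward vector.
; Hard-coded delays time both effects after the attack starts.
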(event `FireProjecti2`
  (`KismetSystemLibrary.Delay` 0.562)
  (`GameplayStatics.ApplyRadialDamage` (`self.MeleeDmg`) (`SceneComponent.K2_GetComponentLocation` (`self.Box2`)) 100.0 (`self.DamageTypeClass`) (`|MakeArray` self :!type "Actor Object Reference") self))

(event `FireProjectil`
  (bind _box1 (`self.Box1`))
  (bind _returnvalue (`SceneComponent.K2_GetComponentRotation` _box1))
  (`KismetSystemLibrary.Delay` 1.493)
  (bind _returnvalue_2 (`|SpawnActorFromClass` "/Game/Mods/Digivolved/Digimon/Agumon/BPS/Proj/ProjSnow_SnowAgumon.ProjSnow_SnowAgumon_C" (`KismetMathLibrary.MakeTransform` (`SceneComponent.K2_GetComponentLocation` _box1) _returnvalue)))
  (`ShooterProjectile.BPInitVelocity` _returnvalue_2 (`KismetMathLibrary.GetForwardVector` _returnvalue)))

(fn `BPDoAttack`
  (params (AttackIndex :type Integer))
  (if (== AttackIndex 1)
    (`self.FireProjectil`)
    (elif (== AttackIndex 0)
      (`self.FireProjecti2`))))

(fn `UserConstructionScript`
  (`parent.UserConstructionScript`))