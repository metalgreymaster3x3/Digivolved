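; Tokomon character Blueprint that adds a melee attack for the Digimon creature.
; BPDoAttack routes the first attack index to a custom event, which waits briefly and then applies radial melee damage around the Box1 component's location, ignoring itself.
; The event keeps a projectile-firing name but spawns no projectile, and the construction script only calls the parent.
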(event `FireProjectil_Copy`
  (`KismetSystemLibrary.Delay` 0.3)
  (`GameplayStatics.ApplyRadialDamage` (`self.Melee Damage`) (`SceneComponent.K2_GetComponentLocation` (`self.Box1`)) 100.0 (`self.Melee_DamageType`) (`|MakeArray` self :!type "Actor Object Reference") self))

(fn `BPDoAttack`
  (params (AttackIndex :type Integer))
  (if (== AttackIndex 0)
    (`self.FireProjectil_Copy`)))

(fn `UserConstructionScript`
  (`parent.UserConstructionScript`))