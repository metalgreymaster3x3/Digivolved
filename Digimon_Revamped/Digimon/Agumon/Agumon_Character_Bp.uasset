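; Agumon Digimon character Blueprint that animates its face and death, and drops a Digicore when a tamed one dies.
; BeginPlay runs a randomized blink loop by swapping eye materials.
; One roll in five makes a tamed Agumon without raw meat play an angry snack montage with movement locked; on that roll, an untamed one exits the loop.
; OnSetDeath plays a replicated death montage, then calls SpawnCore.
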(event `self.BP_OnSetDeath`
  (`self.PlayAnimEx` "/Game/Mods/Digivolved/Digimon_Revamped/Digimon/Agumon/Anims/Montages/Agumonnew_GRP_joint_death_Montage.Agumonnew_GRP_joint_death_Montage" 1.0 "None" true true false false false 0.1)
  (`self.SpawnCore`))

(event `self.ReceiveBeginPlay`
  (bind _angry (`self.Angry`))
  (bind _mesh (`self.Mesh`))
  (bind _mesh_2 (`self.Mesh`))
  (bind _mesh_3 (`self.Mesh`))
  (bind _eyesclosed (`self.EyesClosed`))
  (bind _eyesopen (`self.Eyesopen`))
  (`KismetSystemLibrary.Delay` (`KismetMathLibrary.RandomFloatInRange` 0.1 0.5) :!label _label)
  (`PrimitiveComponent.SetMaterial` _mesh_3 0 _eyesclosed)
  (`PrimitiveComponent.SetMaterial` _mesh_3 1 _eyesclosed)
  (switch `int` (`KismetMathLibrary.RandomIntegerInRange` 0 4)
    (:`0`
      (if (`self.BPIsTamed`)
        (bind _returnvalue (`PrimalInventoryComponent.GetItemTemplateQuantity` (`self.MyInventoryComponent`) "/Game/PrimalEarth/CoreBlueprints/Items/Consumables/PrimalItemConsumable_RawMeat.PrimalItemConsumable_RawMeat_C" null true false false))
        (if (not (>= (`KismetMathLibrary.Conv_IntToDouble` _returnvalue) 1.0))
          (bind _returnvalue_2 (`self.PlayAnimMontage` "/Game/Mods/Digivolved/Digimon_Revamped/Digimon/Agumon/Anims/Montages/Agumonnew_GRP_joint_snacktime_Montage.Agumonnew_GRP_joint_snacktime_Montage"))
          (`PrimitiveComponent.SetMaterial` _mesh 0 _angry)
          (`PrimitiveComponent.SetMaterial` _mesh 1 _angry)
          (set `self.bPreventMovement` true)
          (`KismetSystemLibrary.Delay` _returnvalue_2)
          (set `self.bPreventMovement` false))
        (`KismetSystemLibrary.Delay` (`KismetMathLibrary.RandomFloatInRange` 1.0 5.0) :!label _label_2)
        (`PrimitiveComponent.SetMaterial` _mesh_2 0 _eyesopen)
        (`PrimitiveComponent.SetMaterial` _mesh_2 1 _eyesopen)
        (goto _label)))
    (:`1`
      (goto _label_2))
    (:`2`
      (goto _label_2))
    (:`3`
      (goto _label_2))
    (:`4`
      (goto _label_2))))

(fn `SpawnCore`
  (if (`self.BPIsTamed`)
    (`|SpawnActorFromClass` "/Game/Mods/Digivolved/Digimon_Revamped/Visual_fx/Lifeorb/Digi-core.Digi-core_C" (`KismetMathLibrary.MakeTransform` (`self.K2_GetActorLocation`)) true self)))

(fn `UserConstructionScript`
  (`parent.UserConstructionScript`))