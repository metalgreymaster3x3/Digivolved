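; Digimon creature character for an ARK mod, adding digivolution to a tameable dino.
; A multi-use wheel submenu, hidden for babies until adulthood if allowed, offers up to four target forms to the same team.
; Choosing one at full age spawns a helper actor with the target class and a difficulty-scaled level requirement.
; BeginPlay handles baby spawns and auto-partner buffing, and tamed deaths spawn a Digicore.
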(event Custom|MC_Digivolution1
  (if (== (Variables|Default|GetBabyAge) 1.0)
    (Game|SpawnActorfromClass "/Game/Mods/Digivolved/Digimon_Revamped/Digivolution_logic/digivolve_test/SpawnActor_Digi_to_Digi.SpawnActor_Digi_to_Digi_C" (Transformation|GetActorTransform) true (Utilities|Array|Get(acopy) (Variables|Digivolution|GetDigivolutionarray) (Variables|Digivolution|Getdigivolveoption)) (Variables|Digivolution|GetDigivolveLevelBase) self)))

(event EventBeginPlay
  (bind _asshootergamemode (Utilities|Casting|CastToShooterGameMode (Game|GetGameMode)))
  (CallFunction|GetDigilevel _asshootergamemode)
  (bind _returnvalue (Class|PrimalCharacter|HasBuff "/Game/Mods/Digivolved/Digimon_Revamped/Buffs/Buff_Awakened.Buff_Awakened_C" false))
  (Variables|Default|SetIsAwakened _returnvalue)
  (if (Variables|Default|GetSpawnAsBaby)
    (Class|PrimalDinoCharacter|SetBabyAge 0.0)
    (Variables|Digivolution|SetHideDigivolutions true))
  (if (not (Variables|Default|GetIsAwakened))
    (Utilities|FlowControl|Delay 0.1)
    (if (Variables|Default|GetPartneronspawn)
      (if (Class|PrimalDinoCharacter|BPIsTamed)
        (Class|PrimalBuff|StaticAddBuff "/Game/Mods/Digivolved/Digimon_Revamped/Buffs/Buff_Partnered.Buff_Partnered_C" self 0 0 false)
        (Variables|Default|SetIsPartnered true)))))

(event EventOnSetDeath
  (CallFunction|SpawnCore))

(fn ConstructionScript
  (|CallParentFunction))

(fn SpawnCore
  (if (Class|PrimalDinoCharacter|BPIsTamed)
    (Game|SpawnActorfromClass :Class "/Game/Mods/Digivolved/Digimon_Revamped/Visual_fx/Lifeorb/Digi-core.Digi-core_C" :SpawnTransform (Math|Transform|MakeTransform (Transformation|GetActorLocation)) :SpawnEvenIfColliding true :Old%20Self self)))

(fn BPGetMultiUseEntries
  (params (ForPC :type Player%20Controller%20Object%20Reference) (MultiUseEntries :type Array%20of%20Multi%20Use%20Entry%20Structures))
  (bind _digivolutionarray (Variables|Digivolution|GetDigivolutionarray))
  (bind _digivolutionnames (Variables|Digivolution|GetDigivolutionNames))
  (Variables|Default|SetReturnUseEntries MultiUseEntries)
  (if (== (Variables|/Script/Engine.Actor|GetTargetingTeam ForPC) (Variables|Default|GetTargetingTeam))
    (if (Variables|Digivolution|GetHideDigivolutions)
      _
      (else
        (Utilities|Array|Add (Variables|Default|GetReturnUseEntries) (Utilities|Struct|MakeMultiUseEntry 0 (Utilities|String|Append "Digivolution Menu " (Utilities|String|ToString(Text) (Utilities|Text|FormatText "must be level {Level} to Digivolve" (Utilities|Text|ToText(Integer) (Variables|Digivolution|GetDigivolveLevelBase))))) 160000 -16000 false false false false false false false false true false false true))
        (Utilities|Array|Add (Variables|Default|GetReturnUseEntries) (Utilities|Struct|MakeMultiUseEntry 0 "Back" 160001 -16000 false false false false false false false false true false false true false 300))
        (if (Utilities|ClassIsChildOf (Utilities|Array|Get(acopy) _digivolutionarray) "/Script/ShooterGame.PrimalDinoCharacter")
          (Utilities|Array|Add (Variables|Default|GetReturnUseEntries) (Utilities|Struct|MakeMultiUseEntry 0 (Utilities|String|Append "Digivolve to " (Utilities|Array|Get(acopy) _digivolutionnames)) 170000 -16001 false false false false false false false false false false false false false 300 "(B=175,G=175,R=175,A=255)" "(B=255,G=255,R=255,A=255)" 1.5 1.5))
          (if (Utilities|ClassIsChildOf (Utilities|Array|Get(acopy) _digivolutionarray 1) "/Script/ShooterGame.PrimalDinoCharacter")
            (Utilities|Array|Add (Variables|Default|GetReturnUseEntries) (Utilities|Struct|MakeMultiUseEntry 0 (Utilities|String|Append "Digivolve to " (Utilities|Array|Get(acopy) _digivolutionnames 1)) 170001 16002 false false false false false false false false false false false false false 300 "(B=175,G=175,R=175,A=255)" "(B=255,G=255,R=255,A=255)" 1.5 1.5)))
          (if (Utilities|ClassIsChildOf (Utilities|Array|Get(acopy) _digivolutionarray 2) "/Script/ShooterGame.PrimalDinoCharacter")
            (Utilities|Array|Add (Variables|Default|GetReturnUseEntries) (Utilities|Struct|MakeMultiUseEntry 0 (Utilities|String|Append "Digivolve to " (Utilities|Array|Get(acopy) _digivolutionnames 2)) 170002 -16002 false false false false false false false false false false false false false 300 "(B=175,G=175,R=175,A=255)" "(B=255,G=255,R=255,A=255)" 1.5 1.5)))
          (if (Utilities|ClassIsChildOf (Utilities|Array|Get(acopy) _digivolutionarray 3) "/Script/ShooterGame.PrimalDinoCharacter")
            (Utilities|Array|Add (Variables|Default|GetReturnUseEntries) (Utilities|Struct|MakeMultiUseEntry 0 (Utilities|String|Append "Digivolve to " (Utilities|Array|Get(acopy) _digivolutionnames 3)) 170003 -16003 false false false false false false false false false false false false false 300 "(B=175,G=175,R=175,A=255)" "(B=255,G=255,R=255,A=255)" 1.5 1.5)))
          (else
            (Utilities|Array|Add (Variables|Default|GetReturnUseEntries) (Utilities|Struct|MakeMultiUseEntry 0 "Digivolutions unavailable" 170002 -16002 false true false false false false false false false false false false false 300 "(B=175,G=175,R=175,A=255)" "(B=255,G=255,R=255,A=255)" 0.0 0.0))))))
    (return (Variables|Default|GetReturnUseEntries))))

(fn BPTryMultiUse
  (params (ForPC :type Player%20Controller%20Object%20Reference) (UseIndex :type Integer))
  (bind _asshooterplayercontroller (Utilities|Casting|CastToShooterPlayerController ForPC))
  (switch int UseIndex
    (:Default
      (switch int UseIndex
        (:Default
          _)
        (:120
          (Class|PrimalDinoCharacter|BPNotifyNameEditText _asshooterplayercontroller))))
    (:170000
      (Variables|Digivolution|Setdigivolveoption 0)
      (CallFunction|MCDigivolution1 :!label _label))
    (:170001
      (Variables|Digivolution|Setdigivolveoption 1)
      (goto _label))
    (:170002
      (Variables|Digivolution|Setdigivolveoption 2)
      (goto _label))
    (:170003
      (Variables|Digivolution|Setdigivolveoption 3)
      (goto _label)))
  (return false))

(fn BPClientDoMultiUse
  (params (ForPC :type Player%20Controller%20Object%20Reference) (ClientUseIndex :type Integer))
  (bind _asshooterplayercontroller (Utilities|Casting|CastToShooterPlayerController ForPC))
  (switch int ClientUseIndex
    (:160000
      (LocalVariables|SetCategory 300))
    (:160001
      (LocalVariables|SetCategory 0)))
  (Class|ShooterPlayerController|SetMultiUseWheelCategory _asshooterplayercontroller (LocalVariables|GetCategory)))

(fn Multiuse
  (params (MUEntry :type Array%20of%20Multi%20Use%20Entry%20Structures))
  (bind (_array_element _array_index) (Utilities|Array|ForEachLoopwithBreak MUEntry :!label _label)
    (:LoopBody
      (if (== (.UseIndex (Utilities|Struct|BreakMultiUseEntry _array_element)) 1252)
        (Utilities|Array|SetArrayElem MUEntry _array_index (Utilities|Struct|MakeMultiUseEntry (.ForComponent (Utilities|Struct|BreakMultiUseEntry (Utilities|Array|Get(acopy) MUEntry _array_index))) "Log Data" (.UseIndex (Utilities|Struct|BreakMultiUseEntry (Utilities|Array|Get(acopy) MUEntry _array_index))) (.Priority (Utilities|Struct|BreakMultiUseEntry (Utilities|Array|Get(acopy) MUEntry _array_index))) (.bHideFromUI (Utilities|Struct|BreakMultiUseEntry (Utilities|Array|Get(acopy) MUEntry _array_index))) (.bDisableUse (Utilities|Struct|BreakMultiUseEntry (Utilities|Array|Get(acopy) MUEntry _array_index))) (.bHideActivationKey (Utilities|Struct|BreakMultiUseEntry (Utilities|Array|Get(acopy) MUEntry _array_index))) (.bRepeatMultiUse (Utilities|Struct|BreakMultiUseEntry (Utilities|Array|Get(acopy) MUEntry _array_index))) (.bDisplayOnInventoryUI (Utilities|Struct|BreakMultiUseEntry (Utilities|Array|Get(acopy) MUEntry _array_index))) (.bDisplayOnInventoryUISecondary (Utilities|Struct|BreakMultiUseEntry (Utilities|Array|Get(acopy) MUEntry _array_index))) (.bHarvestable (Utilities|Struct|BreakMultiUseEntry (Utilities|Array|Get(acopy) MUEntry _array_index))) (.bIsSecondaryUse (Utilities|Struct|BreakMultiUseEntry (Utilities|Array|Get(acopy) MUEntry _array_index))) (.bPersistWheelOnActivation (Utilities|Struct|BreakMultiUseEntry (Utilities|Array|Get(acopy) MUEntry _array_index))) (.bOverrideUseTextColor (Utilities|Struct|BreakMultiUseEntry (Utilities|Array|Get(acopy) MUEntry _array_index))) (.bDisplayOnInventoryUITertiary (Utilities|Struct|BreakMultiUseEntry (Utilities|Array|Get(acopy) MUEntry _array_index))) (.bClientSideOnly (Utilities|Struct|BreakMultiUseEntry (Utilities|Array|Get(acopy) MUEntry _array_index))) (.bPersistWheelRequiresDirectActivation (Utilities|Struct|BreakMultiUseEntry (Utilities|Array|Get(acopy) MUEntry _array_index))) (.WheelCategory (Utilities|Struct|BreakMultiUseEntry (Utilities|Array|Get(acopy) MUEntry _array_index))) (.DisableUseColor (Utilities|Struct|BreakMultiUseEntry (Utilities|Array|Get(acopy) MUEntry _array_index))) (.UseTextColor (Utilities|Struct|BreakMultiUseEntry (Utilities|Array|Get(acopy) MUEntry _array_index))) (.EntryActivationTimer (Utilities|Struct|BreakMultiUseEntry (Utilities|Array|Get(acopy) MUEntry _array_index))) (.DefaultEntryActivationTimer (Utilities|Struct|BreakMultiUseEntry (Utilities|Array|Get(acopy) MUEntry _array_index))) (.ActivationSound (Utilities|Struct|BreakMultiUseEntry (Utilities|Array|Get(acopy) MUEntry _array_index)))))
        (goto _label Break)))
    (:Completed
      (return MUEntry))))

(fn BPBecomeAdult
  (if (Variables|Digivolution|GetAdultcandigivolve)
    (Variables|Digivolution|SetHideDigivolutions false)))

(fn GetDigilevel
  (params (self2 :type Shooter%20Game%20Mode%20Object%20Reference))
  (bind _returnvalue (Class|ShooterGameMode|GetFloatOptionIni self2 "" "DifficultyOffset"))
  (if (> _returnvalue 1.0)
    (Variables|Digivolution|SetDigivolveLevelBase (* (Math|Float|Round (* _returnvalue 2.0)) (Variables|Digivolution|GetDigivolveLevelBase))))
  (return))