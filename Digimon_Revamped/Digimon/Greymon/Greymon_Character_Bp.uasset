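; Greymon dino character Blueprint that handles eye blinking and landing animations.
; While alive, it loops from BeginPlay, swapping the eye material at random intervals to blink.
; Switching to Walking plays the landing montage after jump or non-climbable ground-trace checks, shaking a locally controlled rider's camera; falling briefly suppresses this.
; OnLanded and the landing-start notify play the montage directly, bypassing those guards.
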(event `self.ReceiveBeginPlay`
  (bind _mesh (`self.Mesh`))
  (bind _mesh_2 (`self.Mesh`))
  (bind _eyesclosed (`self.EyesClosed`))
  (bind _eyesopen (`self.Eyesopen`))
  (if (not (`self.bIsDead`)) :!label _label
    (`KismetSystemLibrary.Delay` (`KismetMathLibrary.RandomFloatInRange` 1.0 3.0))
    (`PrimitiveComponent.SetMaterial` _mesh_2 1 _eyesclosed)
    (`PrimitiveComponent.SetMaterial` _mesh_2 1 _eyesclosed)
    (`KismetSystemLibrary.Delay` (`KismetMathLibrary.RandomFloatInRange` 0.1 0.5))
    (`PrimitiveComponent.SetMaterial` _mesh 1 _eyesopen)
    (`PrimitiveComponent.SetMaterial` _mesh 1 _eyesopen)
    (goto _label)))

(event `PreventLandingAnimBriefly`
  (set `self.bAllowPlayLandingAnim` false)
  (`KismetSystemLibrary.RetriggerableDelay` 0.2)
  (set `self.bAllowPlayLandingAnim` true))

(fn `BP_OnStartLandingNotify`
  (`self.PlayAnimMontage` (`self.Ref_LandingMontage`)))

(fn `BPon MovementMode Change Notify`
  (`parent.BPOnMovementModeChangedNotify` "MOVE_None" 0)
  (switch `EngineTypes.EMovementMode` (`CharacterMovementComponent.MovementMode` (`self.CharacterMovement`))
    (:`MOVE_Walking`
      (set `self.canCheckAnims` true)
      (`self.Manual Play Land anim`))
    (:`MOVE_Falling`
      (`self.PreventLandingAnimBriefly`))))

(fn `Is Dino Above Ground`
  (params (checkDistance :type "Float (double-precision)"))
  (returns (Result :type Boolean))
  (bind _returnvalue (`KismetMathLibrary.NegateVector` (`self.GetActorUpVector`)))
  (bind _returnvalue_2 (+ (`self.K2_GetActorLocation`) (* _returnvalue (`CapsuleComponent.CapsuleRadius` (`self.CapsuleComponent`)))))
  (bind _returnvalue_3 (+ _returnvalue_2 (* _returnvalue checkDistance)))
  (if (`self.bDebugGreymon`)
    (`KismetSystemLibrary.DrawDebugLine` _returnvalue_2 _returnvalue_3 (struct :`R` 0.266063 :`G` 1.0 :`A` 1.0) 0.1 10.0))
  (bind (_outhit _returnvalue_4) (`VictoryCore.VTraceSingleBP` (`self.K2_GetWorld`) _returnvalue_2 _returnvalue_3 "ECC_GameTraceChannel11"))
  (set `self.RetVal` _returnvalue_4)
  (if (not (not _returnvalue_4))
    (set `self.RetVal` (not (`self.IsNormalClimbable` (`.Normal` (`GameplayStatics.BreakHitResult` _outhit)))))
    (return (or (`self.RetVal`) (and (`|EnumEquality` (`CharacterMovementComponent.MovementMode` (`self.CharacterMovement`)) "MOVE_Walking") (not (`self.bRestoringToLatched`)))))))

(fn `Is Dino Grounded`
  (returns (Result :type Boolean))
  (return (`|EnumEquality` (`CharacterMovementComponent.MovementMode` (`self.CharacterMovement`)) "MOVE_Walking")))

(fn `IsNormalClimbable`
  (params (Normal :type "Object.Vector Structure"))
  (returns (Result :type Boolean))
  (bind _returnvalue (`KismetMathLibrary.Dot_VectorVector` Normal (0.0 0.0 1.0)))
  (return (and (< _returnvalue (`self.requiredNormalDotToClimb_MAX`)) (> _returnvalue (`self.requiredNormalDotToClimb_MIN`)) (< (`KismetMathLibrary.Dot_VectorVector` Normal (`self.GetActorForwardVector`)) 0.0))))

(fn `Manual Play Land anim`
  (bind _ref_landingmontage (`self.Ref_LandingMontage`))
  (bind _rider (`self.Rider`))
  (if (`self.bAllowPlayLandingAnim`)
    (`|ExecutionSequence`
      (:`then_0`
        (bind _returnvalue (`self.GetCurrentMontage`))
        (if (!= _returnvalue _ref_landingmontage)
          (if (`self.CanJumpInternal`)
            (`self.PlayAnimMontage` _ref_landingmontage :!label _label)
            (if (`self.IsLocallyControlled`)
              (`/Engine/EditorBlueprintResources/StandardMacros.IsValid` _rider
                (:`Is Valid`
                  (bind _asshooterplayercontroller (cast `ShooterPlayerController` (`self.GetController` _rider)))
                  (`PlayerController.ClientStartCameraShake` _asshooterplayercontroller "/Game/PrimalEarth/General/HurtCameraShake.HurtCameraShake_C" 5.0 "CameraLocal" (`KismetMathLibrary.Conv_VectorToRotator` (`self.GetActorForwardVector`)) 0.8))))
            (else
              (bind _result (`self.Is Dino Above Ground` 10.0))
              (if _result
                (goto _label))))))
      (:`then_1`
        (if (`self.bDebugGreymon`)
          (`KismetSystemLibrary.PrintString` "LAND" true true (struct :`G` 0.565 :`B` 0.021429 :`A` 1.0)))))))

(fn `OnLanded`
  (params (Hit :type "EngineTypes.HitResult Structure (by ref)"))
  (`self.PlayAnimMontage` (`self.Ref_LandingMontage`))
  (return))

(fn `UserConstructionScript`
  (`parent.UserConstructionScript`))