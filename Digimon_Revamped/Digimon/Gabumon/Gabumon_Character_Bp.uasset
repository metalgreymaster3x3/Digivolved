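; Gabumon character Blueprint, a child class that adds blinking eyes and a death hook.
; BeginPlay runs an endless blink loop, swapping the first two mesh materials between open and closed eyes after randomized delays.
; Each loop pass also clears PreventMovement shortly after the eyes open.
; OnSetDeath calls SpawnCore, which is empty in this Blueprint.
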(event `self.BP_OnSetDeath`
  (`self.SpawnCore`))

(event `self.ReceiveBeginPlay`
  (bind _mesh (`self.Mesh`))
  (bind _mesh_2 (`self.Mesh`))
  (bind _eyesopen (`self.EyesOpen`))
  (bind _eyesclose (`self.EyesClose`))
  (`KismetSystemLibrary.Delay` (`KismetMathLibrary.RandomFloatInRange` 0.1 0.5) :!label _label)
  (`PrimitiveComponent.SetMaterial` _mesh_2 0 _eyesopen)
  (`PrimitiveComponent.SetMaterial` _mesh_2 1 _eyesopen)
  (`KismetSystemLibrary.Delay` 0.2)
  (set `self.bPreventMovement` false)
  (`KismetSystemLibrary.Delay` (`KismetMathLibrary.RandomFloatInRange` 1.0 5.0))
  (`PrimitiveComponent.SetMaterial` _mesh 0 _eyesclose)
  (`PrimitiveComponent.SetMaterial` _mesh 1 _eyesclose)
  (goto _label))

(fn `SpawnCore`)

(fn `UserConstructionScript`
  (`parent.UserConstructionScript`))